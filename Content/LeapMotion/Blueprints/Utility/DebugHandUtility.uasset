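; Debug-draw utility that visualizes Leap Motion hand data relative to its own world location and rotation.
; DebugFullHand draws lower arm and wrist spheres, a palm orientation marker, and joint and tip spheres for all five fingers.
; Helpers rotate offset positions into world space, with scale applied to sphere positions but not to orientation marker origins.
; Orientations render as an arrow with a box at its end; a separate helper shows wrist orientation.
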(fn `DebugFinger`
  (params (Finger :type "AnimFinger Object Reference") (Scale :type "Float (double-precision)" :default 1.0) (Offset :type "Vector Structure"))
  (bind _distal (`AnimFinger.Distal` Finger))
  (bind _position (`AnimBone.Position` _distal))
  (`self.DebugSphereAtActor` (+ _position (* (`KismetMathLibrary.GetForwardVector` (`AnimBone.Orientation` _distal)) (`AnimBone.Length` _distal))) Scale Scale Offset)
  (`self.DebugSphereAtActor` _position Scale Scale Offset)
  (`self.DebugSphereAtActor` (`AnimBone.Position` (`AnimFinger.Intermediate` Finger)) Scale Scale Offset)
  (`self.DebugSphereAtActor` (`AnimBone.Position` (`AnimFinger.Proximal` Finger)) Scale Scale Offset)
  (`self.DebugSphereAtActor` (`AnimBone.Position` (`AnimFinger.Metacarpal` Finger)) Scale Scale Offset))

(fn `DebugFullHand`
  (params (Hand :type "AnimHand Object Reference") (Scale :type "Float (double-precision)" :default 1.0) (Offset :type "Vector Structure" :default (0.0 0.0 0.0)))
  (`self.DebugHand` Hand Scale Offset)
  (`self.DebugFinger` (`AnimHand.Thumb` Hand) Scale Offset)
  (`self.DebugFinger` (`AnimHand.Index` Hand) Scale Offset)
  (`self.DebugFinger` (`AnimHand.Middle` Hand) Scale Offset)
  (`self.DebugFinger` (`AnimHand.Ring` Hand) Scale Offset)
  (`self.DebugFinger` (`AnimHand.Pinky` Hand) Scale Offset))

(fn `DebugHand`
  (params (Hand :type "AnimHand Object Reference") (Scale :type "Float (double-precision)" :default 1.0) (Offset :type "Vector Structure" :default (0.0 0.0 0.0)))
  (locals (WristRadius :type "Float (double-precision)" :default 2.0) (LowerArmRadius :type "Float (double-precision)" :default 4.0) (PalmRadius :type "Float (double-precision)" :default 1.0))
  (bind _palm (`AnimHand.Palm` Hand))
  (`self.DebugSphereAtActor` (`AnimBone.Position` (`AnimHand.LowerArm` Hand)) Scale (`local.LowerArmRadius`) Offset)
  (`self.DebugSphereAtActor` (`AnimBone.Position` (`AnimHand.Wrist` Hand)) Scale (`local.WristRadius`) Offset)
  (`self.DebugOrientationAtRelative` (`AnimBone.Orientation` _palm) (`AnimBone.Position` _palm) Offset 50.0))

(fn `DebugHandOrientation`
  (params (Hand :type "AnimHand Object Reference"))
  (bind _wrist (`AnimHand.Wrist` Hand))
  (`self.DebugOrientation` (`AnimBone.Orientation` _wrist) (+ (`self.K2_GetComponentLocation`) (`AnimBone.Position` _wrist)) 50.0))

(fn `DebugOrientation`
  (params (Orientation :type "Rotator Structure" :default (struct)) (At :type "Vector Structure" :default (0.0 0.0 0.0)) (Scale :type "Float (double-precision)" :default 10.0))
  (bind _returnvalue (`KismetMathLibrary.ComposeRotators` Orientation (`self.K2_GetComponentRotation`)))
  (bind _returnvalue_2 (+ At (* (`KismetMathLibrary.GetForwardVector` _returnvalue) Scale)))
  (`KismetSystemLibrary.DrawDebugArrow` At _returnvalue_2 5.0)
  (`KismetSystemLibrary.DrawDebugBox` _returnvalue_2 (* (0.2 0.2 0.2) Scale) (struct) _returnvalue))

(fn `DebugOrientationAtRelative`
  (params (Orientation :type "Rotator Structure" :default (struct)) (Relative :type "Vector Structure" :default (0.0 0.0 0.0)) (Offset :type "Vector Structure" :default (0.0 0.0 0.0)) (Scale :type "Float (double-precision)" :default 10.0))
  (`self.DebugOrientation` Orientation (+ (`KismetMathLibrary.GreaterGreater_VectorRotator` (+ Offset Relative) (`self.K2_GetComponentRotation`)) (`self.K2_GetComponentLocation`)) Scale))

(fn `DebugSphereAtActor`
  (params (Location :type "Vector Structure" :default (0.0 0.0 0.0)) (Scale :type "Float (double-precision)" :default 1.0) (Radius :type "Float (double-precision)" :default 1.0) (Offset :type "Vector Structure" :default (0.0 0.0 0.0)))
  (`KismetSystemLibrary.DrawDebugSphere` (+ (* (`KismetMathLibrary.GreaterGreater_VectorRotator` (+ Location Offset) (`self.K2_GetComponentRotation`)) Scale) (`self.K2_GetComponentLocation`)) Radius 12 (struct :`A` 1.0)))