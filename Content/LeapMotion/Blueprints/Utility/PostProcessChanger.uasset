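; Leap Motion utility that drives post-process effects on a swappable camera, including VR passthrough.
; Passthrough creates a dynamic material from stereo image and distortion textures, then adds it as a camera blendable with adjustable scalar parameters.
; Color grading, vignette, saturation, fringe and clear functions rebuild the entire post-process settings, overwriting other effects, though color grading keeps vignette.
; SetFringeIntensity actually writes vignette intensity, and FadeIn and FadeOut are empty.
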(event `FadeIn`)

(event `FadeOut`)

(fn `ClearBlendables`
  (set `CameraComponent.PostProcessSettings` (make `PostProcessSettings` :`FilmHealAmount` 0.18 :`BloomIntensity` 1.0 :`BloomThreshold` 1.0 :`Bloom1Size` 1.0 :`Bloom2Size` 4.0 :`Bloom3Size` 16.0 :`Bloom4Size` 32.0 :`Bloom5Size` 100.0 :`Bloom1Tint` (struct :`R` 0.5 :`G` 0.5 :`B` 0.5 :`A` 1.0) :`Bloom2Tint` (struct :`R` 0.5 :`G` 0.5 :`B` 0.5 :`A` 1.0) :`Bloom3Tint` (struct :`R` 0.5 :`G` 0.5 :`B` 0.5 :`A` 1.0) :`Bloom4Tint` (struct :`R` 0.5 :`G` 0.5 :`B` 0.5 :`A` 1.0) :`Bloom5Tint` (struct :`R` 0.5 :`G` 0.5 :`B` 0.5 :`A` 1.0) :`BloomDirtMaskIntensity` 1.0 :`VignetteIntensity` 0.0 :`AmbientOcclusionRadius` 40.0) (`self.PPCamera`)))

(fn `SetCamera`
  (params (NewCamera :type "CameraComponent Object Reference"))
  (set `self.PPCamera` NewCamera))

(fn `SetColorGradingIntensity`
  (params (Value :type "Float (double-precision)" :default 0.0))
  (bind _ppcamera (`self.PPCamera`))
  (set `CameraComponent.PostProcessSettings` (make `PostProcessSettings` :`FilmHealAmount` 0.18 :`BloomIntensity` 1.0 :`BloomThreshold` 1.0 :`Bloom1Size` 1.0 :`Bloom2Size` 4.0 :`Bloom3Size` 16.0 :`Bloom4Size` 32.0 :`Bloom5Size` 100.0 :`Bloom1Tint` (struct :`R` 0.5 :`G` 0.5 :`B` 0.5 :`A` 1.0) :`Bloom2Tint` (struct :`R` 0.5 :`G` 0.5 :`B` 0.5 :`A` 1.0) :`Bloom3Tint` (struct :`R` 0.5 :`G` 0.5 :`B` 0.5 :`A` 1.0) :`Bloom4Tint` (struct :`R` 0.5 :`G` 0.5 :`B` 0.5 :`A` 1.0) :`Bloom5Tint` (struct :`R` 0.5 :`G` 0.5 :`B` 0.5 :`A` 1.0) :`BloomDirtMaskIntensity` 1.0 :`VignetteIntensity` (`.VignetteIntensity` (break `PostProcessSettings` (`CameraComponent.PostProcessSettings` _ppcamera))) :`AmbientOcclusionRadius` 40.0 :`ColorGradingIntensity` (`KismetSystemLibrary.MakeLiteralDouble` Value) :`ColorGradingLUT` "/Engine/EngineResources/Black.Black") _ppcamera))

(fn `SetFringeIntensity`
  (params (Value :type "Float (double-precision)" :default 0.0))
  (set `CameraComponent.PostProcessSettings` (make `PostProcessSettings` :`FilmHealAmount` 0.18 :`BloomIntensity` 1.0 :`BloomThreshold` 1.0 :`Bloom1Size` 1.0 :`Bloom2Size` 4.0 :`Bloom3Size` 16.0 :`Bloom4Size` 32.0 :`Bloom5Size` 100.0 :`Bloom1Tint` (struct :`R` 0.5 :`G` 0.5 :`B` 0.5 :`A` 1.0) :`Bloom2Tint` (struct :`R` 0.5 :`G` 0.5 :`B` 0.5 :`A` 1.0) :`Bloom3Tint` (struct :`R` 0.5 :`G` 0.5 :`B` 0.5 :`A` 1.0) :`Bloom4Tint` (struct :`R` 0.5 :`G` 0.5 :`B` 0.5 :`A` 1.0) :`Bloom5Tint` (struct :`R` 0.5 :`G` 0.5 :`B` 0.5 :`A` 1.0) :`BloomDirtMaskIntensity` 1.0 :`VignetteIntensity` (`KismetSystemLibrary.MakeLiteralDouble` Value) :`AmbientOcclusionRadius` 40.0) (`self.PPCamera`)))

(fn `SetSaturationIntensity`
  (params (Value :type "Float (double-precision)" :default 0.0))
  (bind _returnvalue (`KismetSystemLibrary.MakeLiteralDouble` Value))
  (`/Engine/EditorBlueprintResources/StandardMacros.CompareFloat` _returnvalue
    (:`>`
      (set `CameraComponent.PostProcessSettings` (make `PostProcessSettings` :`FilmSaturation` _returnvalue :`FilmHealAmount` 0.18 :`BloomIntensity` 1.0 :`BloomThreshold` 1.0 :`Bloom1Size` 1.0 :`Bloom2Size` 4.0 :`Bloom3Size` 16.0 :`Bloom4Size` 32.0 :`Bloom5Size` 100.0 :`Bloom1Tint` (struct :`R` 0.5 :`G` 0.5 :`B` 0.5 :`A` 1.0) :`Bloom2Tint` (struct :`R` 0.5 :`G` 0.5 :`B` 0.5 :`A` 1.0) :`Bloom3Tint` (struct :`R` 0.5 :`G` 0.5 :`B` 0.5 :`A` 1.0) :`Bloom4Tint` (struct :`R` 0.5 :`G` 0.5 :`B` 0.5 :`A` 1.0) :`Bloom5Tint` (struct :`R` 0.5 :`G` 0.5 :`B` 0.5 :`A` 1.0) :`BloomDirtMaskIntensity` 1.0 :`AutoExposureMinBrightness` 2.0 :`AutoExposureMaxBrightness` 2.0 :`VignetteIntensity` 0.0 :`AmbientOcclusionRadius` 40.0) (`self.PPCamera`)))
    (:`==`
      (`self.ClearBlendables`))))

(fn `SetVignetteIntensity`
  (params (Value :type "Float (double-precision)" :default 0.0))
  (set `CameraComponent.PostProcessSettings` (make `PostProcessSettings` :`FilmHealAmount` 0.18 :`BloomIntensity` 1.0 :`BloomThreshold` 1.0 :`Bloom1Size` 1.0 :`Bloom2Size` 4.0 :`Bloom3Size` 16.0 :`Bloom4Size` 32.0 :`Bloom5Size` 100.0 :`Bloom1Tint` (struct :`R` 0.5 :`G` 0.5 :`B` 0.5 :`A` 1.0) :`Bloom2Tint` (struct :`R` 0.5 :`G` 0.5 :`B` 0.5 :`A` 1.0) :`Bloom3Tint` (struct :`R` 0.5 :`G` 0.5 :`B` 0.5 :`A` 1.0) :`Bloom4Tint` (struct :`R` 0.5 :`G` 0.5 :`B` 0.5 :`A` 1.0) :`Bloom5Tint` (struct :`R` 0.5 :`G` 0.5 :`B` 0.5 :`A` 1.0) :`BloomDirtMaskIntensity` 1.0 :`VignetteIntensity` (`KismetSystemLibrary.MakeLiteralDouble` Value) :`AmbientOcclusionRadius` 40.0) (`self.PPCamera`)))

(fn `SetVRBlendablePassThrough`
  (params (Left :type "Texture2D Object Reference") (Right :type "Texture2D Object Reference") (LeftDistortion :type "Texture2D Object Reference") (RightDistortion :type "Texture2D Object Reference"))
  ;[1 1 1] Set the Material Instance Parameters
  (bind _returnvalue (`KismetMaterialLibrary.CreateDynamicMaterialInstance` "/LeapMotion/Materials/LeapPassthroughPostProcess.LeapPassthroughPostProcess"))
  (set `self.PPVRMaterialIstance` _returnvalue)
  (`MaterialInstanceDynamic.SetTextureParameterValue` _returnvalue "LeftImage" Left)
  (`MaterialInstanceDynamic.SetTextureParameterValue` _returnvalue "RightImage" Right)
  (`MaterialInstanceDynamic.SetTextureParameterValue` _returnvalue "DistortionLeftImage" LeftDistortion)
  (`MaterialInstanceDynamic.SetTextureParameterValue` _returnvalue "DistortionRightImage" RightDistortion) ; Not used in current material \nimplementation and can be null
  (`CameraComponent.AddOrUpdateBlendable` (`self.PPCamera`) (`self.PPVRMaterialIstance`) 1.0))

(fn `UpdateVRBlendableParameter`
  (params (Parameter :type Name :default "None") (Value :type "Float (double-precision)" :default 0.0))
  (bind _ppvrmaterialistance (`self.PPVRMaterialIstance`))
  (`MaterialInstanceDynamic.SetScalarParameterValue` _ppvrmaterialistance Parameter Value)
  (`CameraComponent.AddOrUpdateBlendable` (`self.PPCamera`) _ppvrmaterialistance 1.0))