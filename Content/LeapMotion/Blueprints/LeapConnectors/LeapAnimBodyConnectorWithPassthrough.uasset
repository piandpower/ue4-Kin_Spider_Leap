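; Leap Motion body connector that adds camera passthrough to a VR headset through a post-process blendable.
; Raw left and right Leap images, with once-fetched distortion maps, link to PostProcessChanger and forward to a parent owner implementing LeapImageLinkInterface.
; A pinch opens a five-second window in which an up or down swipe near the face shows or hides passthrough.
; Functions also toggle image support and mount offset, with an optional debug billboard.
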(event `LeapEventInterface.LeapHandPinched`
  (params (strength :type "Float (single-precision)") (hand :type "LeapHand Object Reference"))
  (set `self.SwipeGestureActive` true)
  (`KismetSystemLibrary.Delay` 5.0)
  (set `self.SwipeGestureActive` false))

(event `LeapEventInterface.SwipeGestureDetected`
  (params (gesture :type "LeapSwipeGesture Object Reference"))
  ;[1 1 1] Passthrough Handling
  (if (`self.SwipeGestureActive`)
    (`/Engine/EditorBlueprintResources/StandardMacros.CompareFloat` (`KismetMathLibrary.VSize` (`LeapSwipeGesture.Position` gesture)) (`self.PassthroughSwipeProximity`) ; Only swipe close to the face
      (:`<`
        (switch `LeapBasicDirection` (`LeapSwipeGesture.BasicDirection` gesture)
          (:`DIRECTION_UP`
            (`self.ShowPassthrough` true))
          (:`DIRECTION_DOWN`
            (`self.ShowPassthrough` false)))
        (set `self.SwipeGestureActive` false)))))

(event `LeapEventInterface.RawImageReceived`
  (params (texture :type "Texture2D Object Reference") (image :type "LeapImage Object Reference"))
  ;[1 1 1] Passthrough Handling
  (`|ExecutionSequence`
    (:`then_0`
      (switch `int` (`LeapImage.Id` image)
        (:`0`
          (set `self.LeftRawImage` texture)
          (if (== (`self.LeftDistortionImage`) null)
            (bind _returnvalue (`LeapImage.Distortion` image))
            (set `self.LeftDistortionImage` _returnvalue)))
        (:`1`
          (set `self.RightRawImage` texture)
          (if (== (`self.RightDistortionImage`) null)
            (bind _returnvalue_2 (`LeapImage.Distortion` image))
            (set `self.RightDistortionImage` _returnvalue_2)))))
    (:`then_1`
      (if (`self.PassthroughLinkInitialized`)
        _
        (elif (and (!= (`self.LeftRawImage`) null) (!= (`self.RightRawImage`) null))
          (`/LeapMotion/Blueprints/Utility/PostProcessChanger.SetVRBlendablePassThrough` (`self.PostProcessChanger`) (`self.LeftRawImage`) (`self.RightRawImage`) (`self.LeftDistortionImage`) (`self.RightDistortionImage`))
          (set `self.PassthroughLinkInitialized` true)
          (`/LeapMotion/Blueprints/Utility/PostProcessChanger.UpdateVRBlendableParameter` (`self.PostProcessChanger`) "Intensity" 0.0)
          (`self.ForwardImageLinksIfSubscribers`)
          ;[1 1 1] Debug
          (if (`self.DebugImages`)
            (`BillboardComponent.SetSprite` (`self.DebugBillboard`) (`self.LeftRawImage`)) ; Debug Images
          ))))))

(event `self.ReceiveBeginPlay`
  (`parent.ReceiveBeginPlay`)
  (`/LeapMotion/Blueprints/Utility/PostProcessChanger.SetCamera` (`self.PostProcessChanger`) (`self.HMD Camera Component`)))

(event `self.SetOwnerLinks`
  (params (HMDCameraOffset :type "Vector Structure") (HMDCameraComponent :type "CameraComponent Object Reference") (UseDefaultIPD :type Boolean) (MeshOffset :type "Vector Structure"))
  (`parent.SetOwnerLinks` HMDCameraOffset HMDCameraComponent UseDefaultIPD MeshOffset)
  (`/LeapMotion/Blueprints/Utility/PostProcessChanger.SetCamera` (`self.PostProcessChanger`) (`self.HMD Camera Component`)))

(fn `EnablePassthrough`
  (params (Enable :type Boolean :default false) (`Enable Swipe Gesture` :type Boolean))
  (bind _leapcontroller (`self.LeapController`))
  (bind _output_get (set `self.PassthroughEnabled` Enable))
  (`LeapController.EnableImageSupport` _leapcontroller _output_get _output_get (`self.UseGammaCorrection`))
  (`LeapController.EnableGesture` _leapcontroller "GESTURE_TYPE_SWIPE" (and _output_get `Enable Swipe Gesture`))
  (set `self.PassthroughLinkInitialized` false) ; Pointers should reinitialize
)

(fn `ForwardImageLinksIfSubscribers`
  (bind _owner (`self.GetImageLinkOwner`))
  (if (!= _owner null)
    (message `/LeapMotion/Blueprints/Interfaces/LeapImageLinkInterface.ImageTextureLinkEstablished` _owner (`self.LeftRawImage`) (`self.RightRawImage`) (`self.LeftDistortionImage`) (`self.RightDistortionImage`))))

(fn `GetImageLinkOwner`
  (returns (Owner :type "Actor Object Reference"))
  (locals (NewLocalVar_0 :type "Interface Class Reference" :default "/LeapMotion/Blueprints/Interfaces/LeapCameraOwnerInterface.LeapCameraOwnerInterface_C"))
  (bind _returnvalue (`ActorComponent.GetOwner` (`self.GetParentComponent`)))
  (if (!= _returnvalue null)
    (if (`KismetSystemLibrary.DoesImplementInterface` _returnvalue "/LeapMotion/Blueprints/Interfaces/LeapImageLinkInterface.LeapImageLinkInterface_C")
      (return _returnvalue)
      (else
        (return null)))
    (else
      (return null))))

(fn `ShowPassthrough`
  (params (Show :type Boolean :default false))
  (bind _postprocesschanger (`self.PostProcessChanger`))
  (if Show
    (`/LeapMotion/Blueprints/Utility/PostProcessChanger.UpdateVRBlendableParameter` _postprocesschanger "Intensity" 1.0) ; Swipe up so we're removing our vr into passthrough
    (else
      (`/LeapMotion/Blueprints/Utility/PostProcessChanger.UpdateVRBlendableParameter` _postprocesschanger "Intensity" 0.0) ; Swipe down back into vr
    )))

(fn `UseMountOffset`
  (params (Use :type Boolean) (Offset :type "Vector Structure" :default (8.0 0.0 0.0)))
  (bind _leapcontroller (`self.LeapController`))
  (if Use
    (`LeapController.SetLeapMountToHMDOffset` _leapcontroller Offset)
    (else
      (`LeapController.SetLeapMountToHMDOffset` _leapcontroller (0.0 0.0 0.0)))))

(fn `UserConstructionScript`
  (bind _debugimages (`self.DebugImages`))
  (bind _debugbillboard (`self.DebugBillboard`))
  (`parent.UserConstructionScript`)
  ;[1 1 1] Hide the debug billboard if we're not debugging
  (`SceneComponent.SetVisibility` _debugbillboard _debugimages false)
  (`SceneComponent.SetHiddenInGame` _debugbillboard (not _debugimages) false))