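; Leap Motion VR character Blueprint that adds passthrough view control to its body connector.
; On BeginPlay it casts the connector to LeapAnimBodyConnectorWithPassthrough, enables passthrough with swipe gesture, and runs console commands for stereo and HMD mirroring.
; An optional F key toggles passthrough through a FlipFlop, which BeginPlay also triggers after a short delay to show it initially.
; Escape exits the game.
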(event `Key|Escape`
  (params (Key :type "Key Structure" :default "AnyKey"))
  (:`Pressed`
    (`KismetSystemLibrary.ExecuteConsoleCommand` "exit")))

(event `Key|F`
  (params (Key :type "Key Structure" :default "AnyKey"))
  (:`Pressed`
    (bind _isa (`/Engine/EditorBlueprintResources/StandardMacros.FlipFlop` :!label _label)
      (:`A`
        _)
      (:`B`
        _))
    (bind _asleap_anim_body_connector_with_passthrough (cast `/LeapMotion/Blueprints/LeapConnectors/LeapAnimBodyConnectorWithPassthrough` (`self.LeapAnimBodyConnector`)))
    (`/LeapMotion/Blueprints/LeapConnectors/LeapAnimBodyConnectorWithPassthrough.ShowPassthrough` _asleap_anim_body_connector_with_passthrough _isa)))

(event `self.ReceiveBeginPlay`
  (`parent.ReceiveBeginPlay`)
  (bind _asleap_anim_body_connector_with_passthrough (cast `/LeapMotion/Blueprints/LeapConnectors/LeapAnimBodyConnectorWithPassthrough` (`self.LeapAnimBodyConnector`)))
  (`/LeapMotion/Blueprints/LeapConnectors/LeapAnimBodyConnectorWithPassthrough.EnablePassthrough` _asleap_anim_body_connector_with_passthrough true true)
  (`|ExecutionSequence`
    (:`then_0`
      (`KismetSystemLibrary.Delay` 0.5)
      (goto _label))
    (:`then_1`
      (`KismetSystemLibrary.ExecuteConsoleCommand` "stereo on")
      (`KismetSystemLibrary.ExecuteConsoleCommand` "hmd mirror mode 1"))))

(fn `UserConstructionScript`
  (`parent.UserConstructionScript`))